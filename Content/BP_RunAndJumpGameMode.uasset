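; Game mode for a run-and-jump game that auto-scrolls a level camera along X at a speed that rises over play time.
; BeginPlay blends the player's view to the first CameraActor found, then binds Upgrade to the OnPlayTimeIncreased dispatcher after the blend delay.
; Tick moves the camera by speed times Level and fires the dispatcher when accumulated time passes Level times ten seconds, incrementing Level.
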(event Custom|Upgrade
  (Math|Integer|IncrementInt (Variables|Default|Getlevel)))

(event EventBeginPlay
  (bind _delaytime (Variables|Default|GetDelayTime))
  (bind _returnvalue (Actor|GetActorOfClass "/Script/Engine.CameraActor"))
  (bind _output_get (Variables|Default|SetCamera _returnvalue))
  (Game|Player|SetViewTargetwithBlend (Game|GetPlayerController 0) _output_get _delaytime "VTBlend_Linear" 0.0 false)
  (Utilities|FlowControl|Delay _delaytime)
  (EventDispatchers|BindEventtoOnPlayTimeIncreased (delegate Custom|Upgrade)))

(event EventTick
  (params (DeltaSeconds :type Float%20%28single-precision%29))
  (Transformation|SetActorLocation (Variables|Default|GetCamera) (+ (Transformation|GetActorLocation (Variables|Default|GetCamera)) (Math|Vector|MakeVector (* DeltaSeconds (Variables|Default|GetCameraSpeed) (Math|Conversions|ToFloat(Integer) (Variables|Default|Getlevel))) 0.0 0.0)) false false)
  (bind _output_get (Variables|Default|SetPlayTime (+ (Variables|Default|GetPlayTime) DeltaSeconds)))
  (if (> _output_get (* (Variables|Default|Getlevel) 1e+01))
    (Default|CallOnPlayTimeIncreased)))

(fn ConstructionScript)