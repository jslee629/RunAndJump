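; BP_JPlayer is a player character Blueprint that adds a sword and death handling to its parent class.
; AttachWeapon spawns a sword, attaches it hidden to the mesh's Hand_Sword socket and stores it as Weapon.
; BeforeDead runs the parent logic, then swaps two mesh material slots to a dissolve material instance.
; AfterDead destroys the weapon before running the parent logic.
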(event EventAfterDead
  (Actor|DestroyActor (Variables|Default|GetWeapon))
  (|CallParentFunction))

(event EventBeforeDead
  (|CallParentFunction)
  (Rendering|Material|SetMaterial (Variables|Character|GetMesh) 0 "/Game/Materials/MI_Dissolve_Inst.MI_Dissolve_Inst")
  (Rendering|Material|SetMaterial (Variables|Character|GetMesh) 1 "/Game/Materials/MI_Dissolve_Inst.MI_Dissolve_Inst"))

(event EventAttachWeapon
  (bind _returnvalue (Game|SpawnActorfromClass "/Game/Character/BP_Sword.BP_Sword_C" (Math|Transform|MakeTransform "0, 0, 0") "AlwaysSpawn" 0 0))
  (Transformation|AttachComponentToComponent _returnvalue (Variables|Character|GetMesh) "Hand_Sword" "KeepRelative" "KeepRelative" "KeepRelative" true)
  (Rendering|SetActorHiddenInGame _returnvalue true)
  (Variables|Default|SetWeapon _returnvalue))

(fn ConstructionScript)